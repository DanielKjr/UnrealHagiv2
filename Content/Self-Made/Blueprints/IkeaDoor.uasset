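; Automatic double glass door that slides open and closed as something enters or leaves its Box1 trigger volume.
; Overlap begin plays the Door1Movement timeline and overlap end reverses it, both only while CutSceneTriggered is false.
; BeginPlay also reverses the timeline, whose update feeds separate vector tracks into MoveComponentTo for GlassDoor1 and GlassDoor2.
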(event `self.ReceiveBeginPlay`
  (bind (_direction _door1_vector _door2_vector) (`Timeline|Door1Movement` :!via `Reverse` :!label _label)
    (:`Update`
      (`|ExecutionSequence`
        (:`then_0`
          (`KismetSystemLibrary.MoveComponentTo` (`self.Glass-Door 1`) _door1_vector))
        (:`then_1`
          (`KismetSystemLibrary.MoveComponentTo` (`self.Glass-Door 2`) _door2_vector))))))

(event `self.Box 1.OnComponentBeginOverlap`
  (params (OverlappedComponent :type "PrimitiveComponent Object Reference") (OtherActor :type "Actor Object Reference") (OtherComp :type "PrimitiveComponent Object Reference") (OtherBodyIndex :type Integer) (bFromSweep :type Boolean) (SweepResult :type "HitResult Structure (by ref)"))
  (if (not (`self.CutSceneTriggered`))
    (goto _label)))

(event `self.Box 1.OnComponentEndOverlap`
  (params (OverlappedComponent :type "PrimitiveComponent Object Reference") (OtherActor :type "Actor Object Reference") (OtherComp :type "PrimitiveComponent Object Reference") (OtherBodyIndex :type Integer))
  (if (not (`self.CutSceneTriggered`))
    (goto _label :!via `Reverse`)))

(fn `UserConstructionScript`)